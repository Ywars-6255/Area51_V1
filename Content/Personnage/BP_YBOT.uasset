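; BP_YBOT is the player character, with movement, crouch, sprint, TPS/FPS camera switching, a flashlight and a backpack inventory.
; Tick drains the flashlight battery through a Delay and switches the light off when empty, while sprint keys start a looping timer that updates endurance.
; AjoutDitem stores items and rebuilds the backpack widget list.
; The pickup input only runs a debug-drawn sphere trace, whose result is unused.
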(event `self.ReceiveTick`
  (params (DeltaSeconds :type "Float (single-precision)"))
  (bind _flashlight_status (`self.FlashLight_Status`))
  (`|ExecutionSequence`
    (:`then_0`
      ;[1 1 1] FlashLight Diminution Battery
      (if _flashlight_status
        (`KismetSystemLibrary.Delay` 0.5)
        (set `self.currBattery` (- (`self.currBattery`) 1.0))))
    (:`then_1`
      (if _flashlight_status
        (if (< (`self.currBattery`) 1.0)
          (set `self.FlashLight_Status` false)
          (`SceneComponent.ToggleVisibility` (`self.SpotLight_parent`) true))))))

(event `InputAction|FlashLight`
  (params (Key :type "Key Structure"))
  (bind _spotlight_parent (`self.SpotLight_parent`))
  ;[1 1 1] FlashLight On / Off
  (:`Pressed`
    (if (`self.FlashLight_Status`)
      (set `self.FlashLight_Status` false)
      (`SceneComponent.ToggleVisibility` _spotlight_parent true)
      (elif (> (`self.currBattery`) 0.0)
        (set `self.FlashLight_Status` true)
        (`SceneComponent.ToggleVisibility` _spotlight_parent true)))))

(event `InputAction|Ramasser`
  (params (Key :type "Key Structure"))
  ;[1 1 1] Ramasser items
  (:`Pressed`
    (`self.Ramasser item`)))

(event `InputAction|Inventaire`
  (params (Key :type "Key Structure"))
  (bind _ui_backpack_ref (`self.UI_Backpack_Ref`))
  ;[1 1 1] Inventaire
  (:`Pressed`
    (`/Engine/EditorBlueprintResources/StandardMacros.IsValid` (`self.UI_Backpack_Ref`)
      (:`Is Valid`
        (`/Engine/EditorBlueprintResources/StandardMacros.FlipFlop`
          (:`A`
            (`Widget.RemoveFromParent` _ui_backpack_ref)
            (set `PlayerController.bShowMouseCursor` false (`GameplayStatics.GetPlayerController` 0)))
          (:`B`
            (`UserWidget.AddToViewport` _ui_backpack_ref 0)
            (`self.Charger inventaire`)
            (set `PlayerController.bShowMouseCursor` true (`GameplayStatics.GetPlayerController` 0) :!label _label))))
      (:`Is Not Valid`
        (bind _returnvalue (`|CreateWidget` "/Game/UI/UI_Backpack.UI_Backpack_C"))
        (bind _output_get (set `self.UI_Backpack_Ref` _returnvalue))
        (`UserWidget.AddToViewport` _output_get 0)
        (`self.Charger inventaire`)
        (goto _label)))))

(event `Key|LeftControl`
  (params (Key :type "Key Structure"))
  ;[1 1 1] Crouch
  (:`Pressed`
    (`self.Crouch`))
  (:`Released`
    (`self.UnCrouch`)))

(event `InputAxis|MoveForward`
  (params (AxisValue :type "Float (single-precision)"))
  ;[1 1 1] Mouvements
  (`self.AddMovementInput` (`KismetMathLibrary.GetForwardVector` (`KismetMathLibrary.MakeRotator` 0.0 0.0 (.yaw (`self.GetControlRotation`)))) AxisValue))

(event `InputAxis|MoveRight`
  (params (AxisValue :type "Float (single-precision)"))
  ;[1 1 1] Mouvements
  (`self.AddMovementInput` (`KismetMathLibrary.GetRightVector` (`KismetMathLibrary.MakeRotator` 0.0 0.0 (.yaw (`self.GetControlRotation`)))) AxisValue))

(event `InputAction|Jump`
  (params (Key :type "Key Structure"))
  ;[1 1 1] Saut
  (:`Pressed`
    (`self.Jump`))
  (:`Released`
    (`self.StopJumping`)))

(event `InputAxis|Turn`
  (params (AxisValue :type "Float (single-precision)"))
  ;[1 1 1] Camera
  (`self.AddControllerYawInput` AxisValue))

(event `Key|LeftShift`
  (params (Key :type "Key Structure"))
  (bind _charactermovement (`self.CharacterMovement`))
  ;[1 1 1] Sprint
  (:`Pressed`
    (set `CharacterMovementComponent.MaxWalkSpeed` 600.0 _charactermovement)
    (`KismetSystemLibrary.K2_SetTimer` null "Gestion_endurance" 0.1 true :!label _label_2))
  (:`Released`
    (set `CharacterMovementComponent.MaxWalkSpeed` 300.0 _charactermovement)
    (goto _label_2)))

(event `InputAxis|LookUp`
  (params (AxisValue :type "Float (single-precision)"))
  ;[1 1 1] Camera
  (`self.AddControllerPitchInput` AxisValue))

(event `InputAction|Switch Caméra`
  (params (Key :type "Key Structure"))
  ;[1 1 1] Camera
  (:`Pressed`
    (`self.Changer caméra`)))

(fn `Ajout d'item`
  (params (Item_Ref :type "/Game/Items/BP_mainitems Object Reference"))
  (`KismetArrayLibrary.Array_Add` (`self.Inventaire`) (`/Game/Items/BP_mainitems.S_items` Item_Ref))
  (`self.K2_DestroyActor` Item_Ref)
  (`self.Charger inventaire`))

(fn `Changer caméra`
  (`ActorComponent.ToggleActive` (`self.Camera TPS`))
  (`ActorComponent.ToggleActive` (`self.Camera FPS`))
  (if (`ActorComponent.IsActive` (`self.Camera FPS`))
    (set `Pawn.bUseControllerRotationYaw` true (`GameplayStatics.GetPlayerPawn` 0))
    (else
      (set `Pawn.bUseControllerRotationYaw` false (`GameplayStatics.GetPlayerPawn` 0))))
  (`SceneComponent.ToggleVisibility` (`self.Mesh`) false))

(fn `Charger inventaire`
  (`PanelWidget.ClearChildren` (`/Game/UI/UI_Backpack.VerticalBox_Bag` (`self.UI_Backpack_Ref`)))
  (for _array_element (`self.Inventaire`)
    (bind _returnvalue (`|CreateWidget` "/Game/UI/UI_items.UI_items_C" null _array_element))
    (`VerticalBox.AddChildToVerticalBox` (`/Game/UI/UI_Backpack.VerticalBox_Bag` (`self.UI_Backpack_Ref`)) _returnvalue)))

(fn `Gestion_endurance`
  (if (`MovementComponent.IsExceedingMaxSpeed` (`self.CharacterMovement`) 300.0)
    (if (> (`self.Endurance`) 0.0)
      ;[1 1 1] baisse de l'endurance
      (set `self.Endurance` (- (`self.Endurance`) 3.0)))
    (elif (< (`self.Endurance`) (`self.Endurance_Max`))
      ;[1 1 1] regene endurance
      (set `self.Endurance` (+ (`self.Endurance`) 3.0)))))

(fn `Ramasser item`
  (bind _camera_tps (`self.Camera TPS`))
  (bind _camera_tps_2 (`self.Camera TPS`))
  (`KismetSystemLibrary.SphereTraceSingle` :`Start` (+ (`SceneComponent.K2_GetComponentLocation` _camera_tps) (* (`SceneComponent.GetForwardVector` _camera_tps) 450.0)) :`End` (+ (`SceneComponent.K2_GetComponentLocation` _camera_tps_2) (* (`SceneComponent.GetForwardVector` _camera_tps_2) 330.0)) :`Radius` 50.0 :`TraceChannel` "TraceTypeQuery1" :`DrawDebugType` "Persistent"))

(fn `UserConstructionScript`)