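; BP_Door is an interactive door that the player opens and closes with the Ouvrir input action.
; A box trigger enables the door's input while a BP_YBOT overlaps it and disables it on exit.
; The input plays or reverses the Ouvrir timeline, which adds a yaw offset to the Porte rotation saved at BeginPlay.
; DoorClosed is updated from that offset to choose the direction.
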(event `self.ReceiveBeginPlay`
  (set `self.Ratation` (`SceneComponent.RelativeRotation` (`self.porte`))))

(event `self.Box.OnComponentBeginOverlap`
  (params (OverlappedComponent :type "PrimitiveComponent Object Reference") (OtherActor :type "Actor Object Reference") (OtherComp :type "PrimitiveComponent Object Reference") (OtherBodyIndex :type Integer) (bFromSweep :type Boolean) (SweepResult :type "HitResult Structure (by ref)"))
  (cast `/Game/Personnage/BP_YBOT` OtherActor)
  (`self.EnableInput` (`GameplayStatics.GetPlayerController` 0)))

(event `InputAction|Ouvrir`
  (params (Key :type "Key Structure"))
  (bind (_ratation_roll _ratation_pitch _ratation_yaw) (`KismetMathLibrary.BreakRotator` (`self.Ratation`)))
  (:`Pressed`
    (if (`self.DoorClosed`)
      (bind (_direction _rotation) (`Timeline|Ouvrir` :!label _label)
        (:`Update`
          (`SceneComponent.K2_SetRelativeRotation` (`self.porte`) (`KismetMathLibrary.MakeRotator` _ratation_roll _ratation_pitch (+ _rotation _ratation_yaw)) false false)
          (set `self.DoorClosed` (< _rotation 1.0))))
      (else
        (goto _label :!via `Reverse`)))))

(event `self.Box.OnComponentEndOverlap`
  (params (OverlappedComponent :type "PrimitiveComponent Object Reference") (OtherActor :type "Actor Object Reference") (OtherComp :type "PrimitiveComponent Object Reference") (OtherBodyIndex :type Integer))
  (cast `/Game/Personnage/BP_YBOT` OtherActor)
  (`self.DisableInput` (`GameplayStatics.GetPlayerController` 0)))

(fn `UserConstructionScript`)