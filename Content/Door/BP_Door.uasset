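; BP_Door is an interactive door that the player toggles open and closed with the Ouvrir input action.
; BoxA enables input on the door while a BP_YBOT overlaps it and disables it on exit.
; A timeline plays or reverses based on IsClosed, adding its yaw offset to the rotation cached at BeginPlay.
; Each timeline update also derives IsClosed from that offset.
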(event `InputAction|Ouvrir`
  (params (Key :type "Key Structure"))
  (:`Pressed`
    (if (`self.isClosed`)
      (bind (_direction _rotation) (`Timeline|Timeline_0` :!label _label)
        (:`Update`
          (`SceneComponent.K2_SetRelativeRotation` (`self.Door`) (`KismetMathLibrary.MakeRotator` (.roll (`self.Rotation`)) (.pitch (`self.Rotation`)) (+ _rotation (.yaw (`self.Rotation`)))) false false)
          (set `self.isClosed` (< _rotation 1.0))))
      (else
        (goto _label :!via `Reverse`)))))

(event `self.ReceiveBeginPlay`
  (set `self.Rotation` (`SceneComponent.RelativeRotation` (`self.Door`))))

(event `self.BoxA.OnComponentBeginOverlap`
  (params (OverlappedComponent :type "PrimitiveComponent Object Reference") (OtherActor :type "Actor Object Reference") (OtherComp :type "PrimitiveComponent Object Reference") (OtherBodyIndex :type Integer) (bFromSweep :type Boolean) (SweepResult :type "HitResult Structure (by ref)"))
  (cast `/Game/Personnage/BP_YBOT` OtherActor)
  (`self.EnableInput` (`GameplayStatics.GetPlayerController` 0)))

(event `self.BoxA.OnComponentEndOverlap`
  (params (OverlappedComponent :type "PrimitiveComponent Object Reference") (OtherActor :type "Actor Object Reference") (OtherComp :type "PrimitiveComponent Object Reference") (OtherBodyIndex :type Integer))
  (cast `/Game/Personnage/BP_YBOT` OtherActor)
  (`self.DisableInput` (`GameplayStatics.GetPlayerController` 0)))

(fn `UserConstructionScript`)